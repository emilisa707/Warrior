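; Gameplay ability that equips the hero's axe, playing the equip montage and ending when it completes, blends out or is interrupted.
; A gameplay event during the montage snaps the carried axe to the right-hand socket and sets it as the current equipped weapon.
; HandleEquipWeapon applies the weapon data: links its anim layer, adds its input mapping context, and grants its abilities, storing the spec handles on the weapon.
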(event `self.K2_ActivateAbility`
  (`AbilityTask_PlayMontageAndWait.CreatePlayMontageAndWaitProxy` "None" "/Game/PlayerCharacters/Montages/AM_Hero_Axe_Equip.AM_Hero_Axe_Equip"
    (:`then`
      (`AbilityTask_WaitGameplayEvent.WaitGameplayEvent` (struct :`TagName` "Player.Event.EquipAxe") null
        (:`EventReceived`
          (`Actor.K2_AttachToComponent` (`PawnCombatComponent.GetCharacterCarriedWeaponByTag` (`self.GetHeroCombatComponentFromActorInfo`) (struct :`TagName` "Player.Weapon.Axe")) (`self.GetOwningComponentFromActorInfo`) "AxeRightHandSocket" "SnapToTarget" "KeepRelative" "KeepWorld" true)
          (`self.HandleEquipWeapon` (`HeroCombatComponent.GetHeroCarriedWeaponByTag` (`self.GetHeroCombatComponentFromActorInfo`) (struct :`TagName` "Player.Weapon.Axe")))
          (set `PawnCombatComponent.CurrentEquippedWeaponTag` (struct :`TagName` "Player.Weapon.Axe") (`self.GetHeroCombatComponentFromActorInfo`)))))
    (:`OnCompleted`
      (`self.K2_EndAbility` :!label _label))
    (:`OnBlendOut`
      (goto _label))
    (:`OnInterrupted`
      (goto _label))
    (:`OnCancelled`
      (goto _label))))

(fn `HandleEquipWeapon`
  (params (InWeaponToEquip :type "WarriorHeroWeapon Object Reference"))
  (locals (CachedHeroWeaponData :type "WarriorHeroWeaponData Structure"))
  (set `local.CachedHeroWeaponData` (`WarriorHeroWeapon.HeroWeaponData` InWeaponToEquip))
  (`|ExecutionSequence`
    (:`then_0`
      (`SkeletalMeshComponent.LinkAnimClassLayers` (`self.GetOwningComponentFromActorInfo`) (`.WeaponAnimLayerToLink` (break `WarriorHeroWeaponData` (`local.CachedHeroWeaponData`)))))
    (:`then_1`
      (`EnhancedInputSubsystemInterface.AddMappingContext` (pcsubsystem `EnhancedInputLocalPlayerSubsystem` (`self.GetHeroControllerFromActorInfo`)) (`.WeaponInputMappingContext` (break `WarriorHeroWeaponData` (`local.CachedHeroWeaponData`))) 1 (struct)))
    (:`then_2`
      (bind _outgrantedabilityspechandles (`WarriorAbilitySystemComponent.GrantHeroWeaponAbilities` (`self.GetWarriorAbilitySystemComponentFromActorInfo`) (`.DefaultWeaponAbilities` (break `WarriorHeroWeaponData` (`local.CachedHeroWeaponData`))) (`self.GetAbilityLevel`)))
      (`WarriorHeroWeapon.AssignGrantedAbilitySpecHandles` (`local.InWeaponToEquip`) _outgrantedabilityspechandles))))